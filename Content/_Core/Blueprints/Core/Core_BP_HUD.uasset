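; Core HUD Blueprint that owns the player's main switcher widget and swaps it out for dialogue with NPCs.
; On BeginPlay it sets game-only input and adds the core switcher widget to the viewport; an event reactivates that switcher's first page.
; Dialogue events create or remove a DemoDialogueWidget, collapsing or restoring the switcher and toggling between UI-only and game-only input.
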(event `self.ReceiveBeginPlay`
  (`WidgetBlueprintLibrary.SetInputMode_GameOnly` (`self.GetOwningPlayerController`))
  (bind _returnvalue (`|CreateWidget` "/Game/_Core/Widgets/WB_Switcher_Core.WB_Switcher_Core_C" (`self.GetOwningPlayerController`)))
  (bind _output_get (set `self.WB Switcher` _returnvalue))
  (`UserWidget.AddToViewport` _returnvalue 0)
  (`UserWidget.AddToViewport` _output_get 0))

(event `Set HUD Widget Active`
  (`WidgetSwitcher.SetActiveWidgetIndex` (`/Game/_Core/Widgets/WB_Switcher_Core.WidgetSwitcher_0` (`self.WB Switcher`)) 0))

(event `Create Dialogue Widget`
  (params (OwningPlayer :type "PlayerController Object Reference") (InDialogue :type "Dialogue Object Reference") (NPCActor :type "Actor Object Reference"))
  (bind _returnvalue (`|CreateWidget` "/DialoguePlugin/UI/DemoDialogueWidget.DemoDialogueWidget_C" OwningPlayer InDialogue NPCActor))
  (`UserWidget.AddToViewport` _returnvalue 0)
  (set `self.Dialogue Widget` _returnvalue)
  (`Widget.SetVisibility` (`self.WB Switcher`) "Collapsed")
  (`WidgetBlueprintLibrary.SetInputMode_UIOnlyEx` (`self.GetOwningPlayerController`) (`self.Dialogue Widget`) "DoNotLock" true))

(event `Remove Dialogue Widget`
  (`Widget.RemoveFromParent` (`self.Dialogue Widget`))
  (`Widget.SetVisibility` (`self.WB Switcher`) "Visible")
  (`WidgetBlueprintLibrary.SetInputMode_GameOnly` (`self.GetOwningPlayerController`) true))

(fn `UserConstructionScript`)
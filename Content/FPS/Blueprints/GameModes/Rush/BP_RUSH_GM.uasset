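; BP_RUSH_GM is the game mode for the FPS Rush mode, switching which player spawns are active as the mode changes phase.
; ActivateSpawns takes the current state and loops through the A and B spawn lists, enabling only spawns whose Phase matches it.
; BeginPlay and the construction script only call their parent implementations.
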(event `self.ReceiveBeginPlay`
  (`parent.ReceiveBeginPlay`))

(event `ActivateSpawns`
  (params (CurrentState :type Integer))
  ;[1 1 1] Activate New Spawns
  (for _array_element (`self.PlayerSpawnsA`)
    (set `/Game/FPS/Blueprints/PlayerSpawn/BP_PlayerSpawn.bActive` (== CurrentState (`/Game/FPS/Blueprints/PlayerSpawn/BP_PlayerSpawn.Phase` _array_element)) _array_element))
  (for _array_element_2 (`self.PlayerSpawnsB`)
    (set `/Game/FPS/Blueprints/PlayerSpawn/BP_PlayerSpawn.bActive` (== CurrentState (`/Game/FPS/Blueprints/PlayerSpawn/BP_PlayerSpawn.Phase` _array_element_2)) _array_element_2)))

(fn `UserConstructionScript`
  (`parent.UserConstructionScript`))
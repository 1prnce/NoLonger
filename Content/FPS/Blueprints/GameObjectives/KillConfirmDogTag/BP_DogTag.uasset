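; Kill Confirmed dog tag pickup that scores when a living character overlaps it.
; On the server, same-team pickups award player score, while other-team pickups also add team points; the game state then removes the tag.
; SetTeam enables collision, and a team RepNotify refreshes material and objective-widget icon color relative to the local player's team.
; A timeline offsets the mesh vertically from its initial position.
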(event `self.ReceiveBeginPlay`
  (bind (_initialposition_x _initialposition_y _initialposition_z) (`KismetMathLibrary.BreakVector` (`self.InitialPosition`)))
  ;[1 1 1] Begin Play
  (bind _asbp_kill_confirmed_gs (cast `/Game/FPS/Blueprints/GameModes/KillConfirmed/BP_KillConfirmed_GS` (`GameplayStatics.GetGameState`)))
  (set `self.GameStateRef` _asbp_kill_confirmed_gs)
  (`self.SetInitialLocation`)
  (`self.UpdateMaterial`)
  (bind (_direction _output) (`Timeline|SetPosition`)
    (:`Update`
      (`SceneComponent.K2_SetRelativeLocation` (`self.StaticMesh`) (`KismetMathLibrary.MakeVector` _initialposition_x _initialposition_y (+ _initialposition_z (* _output 4.0))) false false))))

(event `SetTeam`
  (params (Team :type Integer))
  ;[1 1 1] Set Team
  (set `self.Team` Team)
  (`PrimitiveComponent.SetCollisionEnabled` (`self.Sphere`) "QueryAndPhysics")
  (`self.ForceNetUpdate`))

(event `UpdateMaterial`
  (bind _staticmesh (`self.StaticMesh`))
  ;[1 1 1] Update Material
  (bind _team (message `/Game/FPS/Blueprints/Interfaces/iPlayerState.GetTeam` (`Controller.PlayerState` (`GameplayStatics.GetPlayerController` 0))))
  (if (== _team (`self.Team`))
    (`PrimitiveComponent.SetMaterial` _staticmesh 0 null)
    (bind _dogtagwidgetref (`self.DogtagWidgetRef`)
      (:`then`
        (`self.SetIconColor` _dogtagwidgetref "NewEnumerator3"))
      (:`else`))
    (else
      (`PrimitiveComponent.SetMaterial` _staticmesh 0 null)
      (bind _dogtagwidgetref_2 (`self.DogtagWidgetRef`)
        (:`then`
          (`self.SetIconColor` _dogtagwidgetref_2 "NewEnumerator4"))
        (:`else`)))))

(event `self.Sphere.OnComponentBeginOverlap`
  (params (OverlappedComponent :type "PrimitiveComponent Object Reference") (OtherActor :type "Actor Object Reference") (OtherComp :type "PrimitiveComponent Object Reference") (OtherBodyIndex :type Integer) (bFromSweep :type Boolean) (SweepResult :type "HitResult Structure (by ref)"))
  ;[1 1 1] On Overlap
  (`/Engine/EditorBlueprintResources/ActorMacros.Switch Has Authority`
    (:`Authority`
      (bind _asbp_base_character (cast `/Game/FPS/Blueprints/CharacterAndClasses/BP_BaseCharacter` OtherActor))
      (bind _playerstate (`Pawn.PlayerState` _asbp_base_character))
      (bind _asbp_player_state (cast `/Game/FPS/Blueprints/PlayerState/BP_PlayerState` _playerstate))
      (set `self.PlayerStateRef` _asbp_player_state)
      (if (not (`/Game/FPS/Blueprints/CharacterAndClasses/BP_BaseCharacter.bDead` _asbp_base_character))
        (bind _team (`/Game/FPS/Blueprints/FunctionLibrary/BP_FunctionLibrary.GetPlayerTeamFromPlayerState` _playerstate))
        (if (== (`self.Team`) _team)
          (message `/Game/FPS/Blueprints/Interfaces/iPlayerState.AddScoreToPlayer` (`self.PlayerStateRef`) 50.0 "NewEnumerator15")
          (else
            (`/Game/FPS/Blueprints/GameModes/BP_Base_GS.AddTeamPoints` (`self.GameStateRef`) _team)
            (message `/Game/FPS/Blueprints/Interfaces/iPlayerState.AddScoreToPlayer` (`self.PlayerStateRef`) 50.0 "NewEnumerator14")))
        (`/Game/FPS/Blueprints/GameModes/KillConfirmed/BP_KillConfirmed_GS.RemoveDogTag` (`self.GameStateRef`) self)))))

(fn `OnRep_bTeam`
  (`self.UpdateMaterial`))

(fn `SetInitialLocation`
  (set `self.InitialPosition` (`SceneComponent.RelativeLocation` (`self.StaticMesh`)))
  (bind _aswb_dogtag_icon (cast `` (`WidgetComponent.GetUserWidgetObject` (`self.Widget`))))
  (bind _output_get (set `self.DogtagWidgetRef` _aswb_dogtag_icon))
  (set `/Game/FPS/Blueprints/GameObjectives/KillConfirmDogTag/BP_DogTag.ObjetiveLocation` (`self.K2_GetActorLocation`) _output_get))

(fn `UserConstructionScript`)
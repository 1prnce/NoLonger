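; Team-owned Capture the Flag objective that players steal, drop, return and capture, earning player score and team points.
; Server-side capsule overlap attaches the flag to an enemy's mesh socket; carrier death drops it onto the navmesh.
; A teammate's touch returns a displaced flag home, or captures the carried flag if theirs is at base, with delayed re-activation.
; OnRep of Carrier toggles a HUD icon for the local carrier.
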(event `self.ReceiveBeginPlay`
  ;[1 0.2273 0.1175] BeginPlay
  (`|ExecutionSequence`
    (:`then_0`
      (`/Engine/EditorBlueprintResources/ActorMacros.Switch Has Authority`
        (:`Authority`
          (set `self.InitialPossition` (`self.K2_GetActorLocation`))
          (set `self.InitialRotation` (`self.K2_GetActorRotation`)))))
    (:`then_1`
      (bind _aswb_capture_the_flag_world_widget (cast `` (`WidgetComponent.GetUserWidgetObject` (`self.Widget`))))
      (set `/Game/FPS/Blueprints/GameObjectives/CTF_Flag/BP_BaseFlag.Objective` self _aswb_capture_the_flag_world_widget)
      (set `/Game/FPS/Blueprints/GameObjectives/CTF_Flag/BP_BaseFlag.Team` (`self.Team`) _aswb_capture_the_flag_world_widget))))

(event `self.Capsule.OnComponentBeginOverlap`
  (params (OverlappedComponent :type "PrimitiveComponent Object Reference") (OtherActor :type "Actor Object Reference") (OtherComp :type "PrimitiveComponent Object Reference") (OtherBodyIndex :type Integer) (bFromSweep :type Boolean) (SweepResult :type "HitResult Structure (by ref)"))
  (bind _pawnref (`self.PawnRef`))
  ;[0.01562 0.01562 0.01562] OnOverlap with flag capsule
  (`/Engine/EditorBlueprintResources/ActorMacros.Switch Has Authority`
    (:`Authority`
      (if (`self.bActive`)
        (if (not (`self.bFlagTaken`))
          (bind _asbp_base_character (cast `/Game/FPS/Blueprints/CharacterAndClasses/BP_BaseCharacter` OtherActor))
          (bind _output_get (set `self.PawnRef` _asbp_base_character))
          (if (`/Game/FPS/Blueprints/CharacterAndClasses/BP_BaseCharacter.bDead` _output_get)
            _
            (elif (!= (`/Game/FPS/Blueprints/FunctionLibrary/BP_FunctionLibrary.GetPlayerTeamFromPlayerState` (`Pawn.PlayerState` _asbp_base_character)) (`self.Team`))
              (set `self.bActive` false)
              (set `self.bFlagTaken` true)
              (set `self.Carrier` _pawnref)
              (message `/Game/FPS/Blueprints/Interfaces/iPlayerState.AddScoreToPlayer` (`Pawn.PlayerState` _pawnref) 100.0 "NewEnumerator18")
              (`/Engine/EditorBlueprintResources/StandardMacros.IsValid` _pawnref
                (:`Is Valid`
                  (`self.K2_AttachToComponent` (`Character.Mesh` _pawnref) "FlagSocket" "SnapToTarget" "KeepRelative" "KeepRelative")
                  (`self.SetOwner` _pawnref)
                  (add `/Game/FPS/Blueprints/CharacterAndClasses/BP_BaseCharacter.OnDeath` (`self.PawnRef`) (delegate `OnPlayerDeathEvent`))))
              (else
                ;;[1 1 1] Your Team flag
                (bind _success (`self.TryToAddPoint`))
                (if _success
                  (`KismetSystemLibrary.Delay` 1.0)
                  (set `self.bFlagTaken` false)
                  (remove `/Game/FPS/Blueprints/CharacterAndClasses/BP_BaseCharacter.OnDeath` (`self.PawnRef`) (delegate `OnPlayerDeathEvent`)))))))))))

(event `OnPlayerDeathEvent`
  ;[0.01562 0.01562 0.01562] OnOverlap with flag capsule
  (`self.DropFlag`))

(event `ResetFlag`
  ;[0.01562 0.01562 0.01562] OnOverlap with flag capsule
  (`KismetSystemLibrary.Delay` 1.0)
  (set `self.bActive` true))

(event `DropFlag`
  ;[0.01562 0.01562 0.01562] OnOverlap with flag capsule
  (set `self.Carrier` null)
  (`self.SetOwner` null)
  (`self.K2_DetachFromActor` self "KeepWorld" "KeepWorld" "KeepWorld")
  (set `self.bFlagTaken` false)
  (`self.ResetFlag`)
  (`self.K2_SetActorLocationAndRotation` :`self` self :`NewLocation` (`NavigationSystemV1.K2_ProjectPointToNavigation` (`self.K2_GetActorLocation` self) null null (1000.0 1000.0 1000.0)) :`bTeleport` true)
  (bind _pawnref (`self.PawnRef`)
    (:`then`
      (remove `/Game/FPS/Blueprints/CharacterAndClasses/BP_BaseCharacter.OnDeath` _pawnref (delegate `OnPlayerDeathEvent`)))
    (:`else`)))

(fn `OnRep_Carrier`
  (bind _flag_widgeticon (`self.Flag_WidgetIcon`))
  (bind _carrier (`self.Carrier`)
    (:`then`
      (if (== _carrier (`GameplayStatics.GetPlayerPawn` 0))
        (bind _returnvalue (`|CreateWidget` null (`GameplayStatics.GetPlayerController` 0)))
        (bind _output_get (set `self.Flag_WidgetIcon` _returnvalue))
        (`/Engine/EditorBlueprintResources/StandardMacros.IsValid` _output_get
          (:`Is Valid`
            (`UserWidget.AddToViewport` _output_get 0)))
        (else
          (`/Engine/EditorBlueprintResources/StandardMacros.IsValid` _flag_widgeticon :!label _label
            (:`Is Valid`
              (`Widget.RemoveFromParent` _flag_widgeticon))))))
    (:`else`
      (goto _label))))

(fn `TryToAddPoint`
  (returns (Success :type Boolean))
  (locals (bCarringFlag :type Boolean) (AttachedFlag :type "/Game/FPS/Blueprints/GameObjectives/CTF_Flag/BP_BaseFlag Object Reference"))
  (bind _attachedflag (`local.AttachedFlag`))
  (bind _playerstate (`Pawn.PlayerState` (`self.PawnRef`)))
  (set `local.bCarringFlag` false)
  (for _array_element (`self.GetAttachedActors` (`self.PawnRef`) true false)
    (bind _asbp_base_flag (cast `/Game/FPS/Blueprints/GameObjectives/CTF_Flag/BP_BaseFlag` _array_element))
    (set `local.bCarringFlag` true)
    (set `local.AttachedFlag` _asbp_base_flag))
  (if (and (`local.bCarringFlag`) (<= (`KismetMathLibrary.Abs` (`KismetMathLibrary.VSize` (- (`self.InitialPossition`) (`self.K2_GetActorLocation`)))) 1.0))
    ;[1 1 1] Add points
    (`/Game/FPS/Blueprints/GameModes/BP_Base_GS.AddTeamPoints` (cast `/Game/FPS/Blueprints/GameModes/BP_Base_GS` (`GameplayStatics.GetGameState`) :!pure true) (`/Game/FPS/Blueprints/FunctionLibrary/BP_FunctionLibrary.GetPlayerTeamFromPlayerState` _playerstate))
    (message `/Game/FPS/Blueprints/Interfaces/iPlayerState.AddScoreToPlayer` _playerstate 350.0 "NewEnumerator11")
    ;[1 1 1] ResetFlag
    (set `self.bActive` false)
    (`self.DropFlag` _attachedflag)
    (`self.ResetFlag` _attachedflag)
    (`self.ResetFlag`)
    (bind _attachedflag_2 (`local.AttachedFlag`)
      (:`then`
        (`self.K2_SetActorLocation` _attachedflag_2 (`/Game/FPS/Blueprints/GameObjectives/CTF_Flag/BP_BaseFlag.InitialPossition` _attachedflag_2) false true)
        (`self.ForceNetUpdate`)
        (return true))
      (:`else`))
    (elif (<= (`KismetMathLibrary.Abs` (`KismetMathLibrary.VSize` (- (`self.InitialPossition`) (`self.K2_GetActorLocation`)))) 1.0)
      (return false)
      (else
        (set `self.bActive` false)
        (message `/Game/FPS/Blueprints/Interfaces/iPlayerState.AddScoreToPlayer` (`Pawn.PlayerState` (`self.PawnRef`)) 100.0 "NewEnumerator19")
        (`self.ResetFlag`)
        (`self.K2_TeleportTo` (`self.InitialPossition`) (`self.InitialRotation`))
        (`self.K2_SetActorRotation` (struct) true)
        (return false)))))

(fn `UserConstructionScript`)